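; Player actor that moves across the horizontal plane from left stick input.
; Each Tick it maps stick Y and X to world X and Y, normalizes the vector, and scales it by MovementSpeed and delta time, so analog magnitude is discarded.
; Any non-zero result offsets the actor with sweep and rotates Model via MakeRotFromZ, pointing the model's Z axis along the movement direction.
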(event EventBeginPlay)

(event Collision|EventActorBeginOverlap
  (params (OtherActor :type Actor%20Object%20Reference)))

(event EventTick
  (params (DeltaSeconds :type Float%20%28single-precision%29))
  (bind _returnvalue (Input|AxisValues|GetLeftStickY))
  (bind _returnvalue_2 (Input|AxisValues|GetLeftStickX))
  (bind _movementspeed (Variables|Default|GetMovementSpeed))
  (bind _returnvalue_3 (Math|Vector|MakeVector _returnvalue _returnvalue_2 0.0))
  (bind _returnvalue_4 (* DeltaSeconds _movementspeed))
  (bind _returnvalue_5 (Math|Vector|Normalize _returnvalue_3))
  (bind _returnvalue_6 (* _returnvalue_5 _returnvalue_4))
  (Utilities|FlowControl|Sequence
    (:then_0
      ;[1 1 1] Move Pawn
      (if (> (Math|Vector|VectorLength _returnvalue_6) 0.0)
        (Transformation|SetWorldRotation (Variables|Default|GetModel) (Math|Rotator|MakeRotfromZ _returnvalue_6) false false)
        (Transformation|AddActorWorldOffset _returnvalue_6 true)))))

(fn ConstructionScript)