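; VoronoiRenderer drives a four-player Voronoi split-screen composite for SpinTopCharacter players through a dynamic material on its Plane.
; Each tick it finds the players' bounding area, normalizes their positions into Voronoi site coordinates, and feeds them to the material.
; It offsets each player's SceneCapture2D from their camera, blending toward a snap-selected player's view by distance.
; Pairwise player positions also set the material's dividing line thicknesses.
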(event EventBeginPlay)

(event Collision|EventActorBeginOverlap
  (params (OtherActor :type Actor%20Object%20Reference)))

(event EventTick
  (params (DeltaSeconds :type Float%20%28single-precision%29))
  (CallFunction|CalculateVoronoiBounds)
  (CallFunction|UpdatePlayerCameraPositions))

(fn ConstructionScript
  (bind _returnvalue (Rendering|Material|CreateDynamicMaterialInstance (Variables|Default|GetPlane) 0 "/Game/Materials/Voronoi_Render_Snap_backup.Voronoi_Render_Snap_backup" "None" :!class /Script/Engine.PrimitiveComponent))
  (Variables|Default|SetVoronoi%20Mat _returnvalue)
  (bind _outactors (Actor|GetAllActorsOfClass "VoronoiRenderer_C"))
  (Rendering|Material|SetMaterial (Variables|VoronoiRenderer_C|GetPlane (Utilities|Array|Get(acopy) _outactors)) 0 (Variables|Default|GetVoronoi%20Mat)))

(fn UpdatePlayerCameraPositions
  (bind _voronoi_mat (Variables|Default|GetVoronoi%20Mat))
  (bind _minbound (Variables|Default|GetMinBound))
  (bind (_x _y) (Math|Vector|BreakVector _minbound))
  (bind _outactors (Actor|GetAllActorsOfClass "/Game/Blueprints/SpinTopCharacter.SpinTopCharacter_C"))
  (for _array_element _outactors
    (switch int (Variables|/Game/Blueprints/SpinTopCharacter.SpinTopCharacter_C|GetPlayerId _array_element)
      (:0
        (Variables|Default|SetPlayer1Coord (Math|Vector|MakeVector (/ (- (.Y (Math|Vector|BreakVector (Transformation|GetActorLocation _array_element))) _y) (Variables|Default|GetYSize)) (- 1.0 (/ (- (.X (Math|Vector|BreakVector (Transformation|GetActorLocation _array_element))) _x) (Variables|Default|GetXSize))) 0.0))
        (Variables|Default|SetPlayer1Pos (Transformation|GetActorLocation _array_element))
        (Variables|Default|SetPlayer1CamPos (Transformation|GetWorldLocation (Actor|GetComponentbyClass _array_element "/Script/Engine.CameraComponent"))))
      (:1
        (Variables|Default|SetPlayer2Coord (Math|Vector|MakeVector (/ (- (.Y (Math|Vector|BreakVector (Transformation|GetActorLocation _array_element))) _y) (Variables|Default|GetYSize)) (- 1.0 (/ (- (.X (Math|Vector|BreakVector (Transformation|GetActorLocation _array_element))) _x) (Variables|Default|GetXSize))) 0.0))
        (Variables|Default|SetPlayer2Pos (Transformation|GetActorLocation _array_element))
        (Variables|Default|SetPlayer2CamPos (Transformation|GetWorldLocation (Actor|GetComponentbyClass _array_element "/Script/Engine.CameraComponent"))))
      (:2
        (Variables|Default|SetPlayer3Coord (Math|Vector|MakeVector (/ (- (.Y (Math|Vector|BreakVector (Transformation|GetActorLocation _array_element))) _y) (Variables|Default|GetYSize)) (- 1.0 (/ (- (.X (Math|Vector|BreakVector (Transformation|GetActorLocation _array_element))) _x) (Variables|Default|GetXSize))) 0.0))
        (Variables|Default|SetPlayer3Pos (Transformation|GetActorLocation _array_element))
        (Variables|Default|SetPlayer3CamPos (Transformation|GetWorldLocation (Actor|GetComponentbyClass _array_element "/Script/Engine.CameraComponent"))))
      (:3
        (Variables|Default|SetPlayer4Coord (Math|Vector|MakeVector (/ (- (.Y (Math|Vector|BreakVector (Transformation|GetActorLocation _array_element))) _y) (Variables|Default|GetYSize)) (- 1.0 (/ (- (.X (Math|Vector|BreakVector (Transformation|GetActorLocation _array_element))) _x) (Variables|Default|GetXSize))) 0.0))
        (Variables|Default|SetPlayer4Pos (Transformation|GetActorLocation _array_element))
        (Variables|Default|SetPlayer4CamPos (Transformation|GetWorldLocation (Actor|GetComponentbyClass _array_element "/Script/Engine.CameraComponent"))))))
  (Rendering|Material|SetScalarParameterValue _voronoi_mat "x1" (.X (Math|Vector|BreakVector (Variables|Default|GetPlayer1Coord))) :!class /Script/Engine.MaterialInstanceDynamic)
  (Rendering|Material|SetScalarParameterValue _voronoi_mat "y1" (.Y (Math|Vector|BreakVector (Variables|Default|GetPlayer1Coord))) :!class /Script/Engine.MaterialInstanceDynamic)
  (Rendering|Material|SetScalarParameterValue _voronoi_mat "x2" (.X (Math|Vector|BreakVector (Variables|Default|GetPlayer2Coord))) :!class /Script/Engine.MaterialInstanceDynamic)
  (Rendering|Material|SetScalarParameterValue _voronoi_mat "y2" (.Y (Math|Vector|BreakVector (Variables|Default|GetPlayer2Coord))) :!class /Script/Engine.MaterialInstanceDynamic)
  (Rendering|Material|SetScalarParameterValue _voronoi_mat "x3" (.X (Math|Vector|BreakVector (Variables|Default|GetPlayer3Coord))) :!class /Script/Engine.MaterialInstanceDynamic)
  (Rendering|Material|SetScalarParameterValue _voronoi_mat "y3" (.Y (Math|Vector|BreakVector (Variables|Default|GetPlayer3Coord))) :!class /Script/Engine.MaterialInstanceDynamic)
  (Rendering|Material|SetScalarParameterValue _voronoi_mat "x4" (.X (Math|Vector|BreakVector (Variables|Default|GetPlayer4Coord))) :!class /Script/Engine.MaterialInstanceDynamic)
  (Rendering|Material|SetScalarParameterValue _voronoi_mat "y4" (.Y (Math|Vector|BreakVector (Variables|Default|GetPlayer4Coord))) :!class /Script/Engine.MaterialInstanceDynamic)
  (for _array_element_2 _outactors
    (switch int (Variables|/Game/Blueprints/SpinTopCharacter.SpinTopCharacter_C|GetPlayerId _array_element_2)
      (:0
        (Transformation|SetWorldLocation (Actor|GetComponentbyClass _array_element_2 "/Script/Engine.SceneCaptureComponent2D") (Math|Vector|Lerp(Vector) (+ (Math|Vector|MakeVector (* (- (.Y (Math|Vector|BreakVector (Utilities|Array|Get(acopy) (Utilities|Array|MakeArray (Variables|Default|GetPlayer1Coord) (Variables|Default|GetPlayer2Coord) (Variables|Default|GetPlayer3Coord) (Variables|Default|GetPlayer4Coord)) (Variables|/Game/Blueprints/SpinTopCharacter.SpinTopCharacter_C|GetPlayerId _array_element_2)))) 0.5) (Variables|Default|GetXCoordinateOffset)) (* (- (- 1.0 (.X (Math|Vector|BreakVector (Utilities|Array|Get(acopy) (Utilities|Array|MakeArray (Variables|Default|GetPlayer1Coord) (Variables|Default|GetPlayer2Coord) (Variables|Default|GetPlayer3Coord) (Variables|Default|GetPlayer4Coord)) (Variables|/Game/Blueprints/SpinTopCharacter.SpinTopCharacter_C|GetPlayerId _array_element_2))))) 0.5) (Variables|Default|GetYCoordinateOffset)) 0.0) (Utilities|Array|Get(acopy) (Utilities|Array|MakeArray (Variables|Default|GetPlayer1CamPos) (Variables|Default|GetPlayer2CamPos) (Variables|Default|GetPlayer3CamPos) (Variables|Default|GetPlayer4CamPos)) (Variables|/Game/Blueprints/SpinTopCharacter.SpinTopCharacter_C|GetPlayerId _array_element_2))) (+ (Math|Vector|MakeVector (* (- (.Y (Math|Vector|BreakVector (Utilities|Array|Get(acopy) (Utilities|Array|MakeArray (Variables|Default|GetPlayer1Coord) (Variables|Default|GetPlayer2Coord) (Variables|Default|GetPlayer3Coord) (Variables|Default|GetPlayer4Coord)) (Class|VoronoiBlueprints|SnaptoClosest (Utilities|Array|MakeArray (Variables|Default|GetPlayer1Pos) (Variables|Default|GetPlayer2Pos) (Variables|Default|GetPlayer3Pos) (Variables|Default|GetPlayer4Pos)) (Utilities|Array|MakeArray (Variables|Default|GetPlayer1Coord) (Variables|Default|GetPlayer2Coord) (Variables|Default|GetPlayer3Coord) (Variables|Default|GetPlayer4Coord)) (Variables|/Game/Blueprints/SpinTopCharacter.SpinTopCharacter_C|GetPlayerId _array_element_2) (Variables|Default|GetSnapDistance))))) 0.5) (Variables|Default|GetXCoordinateOffset)) (* (- (- 1.0 (.X (Math|Vector|BreakVector (Utilities|Array|Get(acopy) (Utilities|Array|MakeArray (Variables|Default|GetPlayer1Coord) (Variables|Default|GetPlayer2Coord) (Variables|Default|GetPlayer3Coord) (Variables|Default|GetPlayer4Coord)) (Class|VoronoiBlueprints|SnaptoClosest (Utilities|Array|MakeArray (Variables|Default|GetPlayer1Pos) (Variables|Default|GetPlayer2Pos) (Variables|Default|GetPlayer3Pos) (Variables|Default|GetPlayer4Pos)) (Utilities|Array|MakeArray (Variables|Default|GetPlayer1Coord) (Variables|Default|GetPlayer2Coord) (Variables|Default|GetPlayer3Coord) (Variables|Default|GetPlayer4Coord)) (Variables|/Game/Blueprints/SpinTopCharacter.SpinTopCharacter_C|GetPlayerId _array_element_2) (Variables|Default|GetSnapDistance)))))) 0.5) (Variables|Default|GetYCoordinateOffset)) 0.0) (Utilities|Array|Get(acopy) (Utilities|Array|MakeArray (Variables|Default|GetPlayer1CamPos) (Variables|Default|GetPlayer2CamPos) (Variables|Default|GetPlayer3CamPos) (Variables|Default|GetPlayer4CamPos)) (Class|VoronoiBlueprints|SnaptoClosest (Utilities|Array|MakeArray (Variables|Default|GetPlayer1Pos) (Variables|Default|GetPlayer2Pos) (Variables|Default|GetPlayer3Pos) (Variables|Default|GetPlayer4Pos)) (Utilities|Array|MakeArray (Variables|Default|GetPlayer1Coord) (Variables|Default|GetPlayer2Coord) (Variables|Default|GetPlayer3Coord) (Variables|Default|GetPlayer4Coord)) (Variables|/Game/Blueprints/SpinTopCharacter.SpinTopCharacter_C|GetPlayerId _array_element_2) (Variables|Default|GetSnapDistance)))) (Class|VoronoiBlueprints|SnapLerpValue (Utilities|Array|Get(acopy) (Utilities|Array|MakeArray (Variables|Default|GetPlayer1Pos) (Variables|Default|GetPlayer2Pos) (Variables|Default|GetPlayer3Pos) (Variables|Default|GetPlayer4Pos)) (Variables|/Game/Blueprints/SpinTopCharacter.SpinTopCharacter_C|GetPlayerId _array_element_2)) (Utilities|Array|Get(acopy) (Utilities|Array|MakeArray (Variables|Default|GetPlayer1Pos) (Variables|Default|GetPlayer2Pos) (Variables|Default|GetPlayer3Pos) (Variables|Default|GetPlayer4Pos)) (Class|VoronoiBlueprints|SnaptoClosest (Utilities|Array|MakeArray (Variables|Default|GetPlayer1Pos) (Variables|Default|GetPlayer2Pos) (Variables|Default|GetPlayer3Pos) (Variables|Default|GetPlayer4Pos)) (Utilities|Array|MakeArray (Variables|Default|GetPlayer1Coord) (Variables|Default|GetPlayer2Coord) (Variables|Default|GetPlayer3Coord) (Variables|Default|GetPlayer4Coord)) (Variables|/Game/Blueprints/SpinTopCharacter.SpinTopCharacter_C|GetPlayerId _array_element_2) (Variables|Default|GetSnapDistance))) (Variables|Default|GetSnapClose) (Variables|Default|GetSnapInterpolation))) false false))
      (:1
        (Transformation|SetWorldLocation (Actor|GetComponentbyClass _array_element_2 "/Script/Engine.SceneCaptureComponent2D") (Math|Vector|Lerp(Vector) (+ (Math|Vector|MakeVector (* (- (.Y (Math|Vector|BreakVector (Utilities|Array|Get(acopy) (Utilities|Array|MakeArray (Variables|Default|GetPlayer1Coord) (Variables|Default|GetPlayer2Coord) (Variables|Default|GetPlayer3Coord) (Variables|Default|GetPlayer4Coord)) (Variables|/Game/Blueprints/SpinTopCharacter.SpinTopCharacter_C|GetPlayerId _array_element_2)))) 0.5) (Variables|Default|GetXCoordinateOffset)) (* (- (- 1.0 (.X (Math|Vector|BreakVector (Utilities|Array|Get(acopy) (Utilities|Array|MakeArray (Variables|Default|GetPlayer1Coord) (Variables|Default|GetPlayer2Coord) (Variables|Default|GetPlayer3Coord) (Variables|Default|GetPlayer4Coord)) (Variables|/Game/Blueprints/SpinTopCharacter.SpinTopCharacter_C|GetPlayerId _array_element_2))))) 0.5) (Variables|Default|GetYCoordinateOffset)) 0.0) (Utilities|Array|Get(acopy) (Utilities|Array|MakeArray (Variables|Default|GetPlayer1CamPos) (Variables|Default|GetPlayer2CamPos) (Variables|Default|GetPlayer3CamPos) (Variables|Default|GetPlayer4CamPos)) (Variables|/Game/Blueprints/SpinTopCharacter.SpinTopCharacter_C|GetPlayerId _array_element_2))) (+ (Math|Vector|MakeVector (* (- (.Y (Math|Vector|BreakVector (Utilities|Array|Get(acopy) (Utilities|Array|MakeArray (Variables|Default|GetPlayer1Coord) (Variables|Default|GetPlayer2Coord) (Variables|Default|GetPlayer3Coord) (Variables|Default|GetPlayer4Coord)) (Class|VoronoiBlueprints|SnaptoClosest (Utilities|Array|MakeArray (Variables|Default|GetPlayer1Pos) (Variables|Default|GetPlayer2Pos) (Variables|Default|GetPlayer3Pos) (Variables|Default|GetPlayer4Pos)) (Utilities|Array|MakeArray (Variables|Default|GetPlayer1Coord) (Variables|Default|GetPlayer2Coord) (Variables|Default|GetPlayer3Coord) (Variables|Default|GetPlayer4Coord)) (Variables|/Game/Blueprints/SpinTopCharacter.SpinTopCharacter_C|GetPlayerId _array_element_2) (Variables|Default|GetSnapDistance))))) 0.5) (Variables|Default|GetXCoordinateOffset)) (* (- (- 1.0 (.X (Math|Vector|BreakVector (Utilities|Array|Get(acopy) (Utilities|Array|MakeArray (Variables|Default|GetPlayer1Coord) (Variables|Default|GetPlayer2Coord) (Variables|Default|GetPlayer3Coord) (Variables|Default|GetPlayer4Coord)) (Class|VoronoiBlueprints|SnaptoClosest (Utilities|Array|MakeArray (Variables|Default|GetPlayer1Pos) (Variables|Default|GetPlayer2Pos) (Variables|Default|GetPlayer3Pos) (Variables|Default|GetPlayer4Pos)) (Utilities|Array|MakeArray (Variables|Default|GetPlayer1Coord) (Variables|Default|GetPlayer2Coord) (Variables|Default|GetPlayer3Coord) (Variables|Default|GetPlayer4Coord)) (Variables|/Game/Blueprints/SpinTopCharacter.SpinTopCharacter_C|GetPlayerId _array_element_2) (Variables|Default|GetSnapDistance)))))) 0.5) (Variables|Default|GetYCoordinateOffset)) 0.0) (Utilities|Array|Get(acopy) (Utilities|Array|MakeArray (Variables|Default|GetPlayer1CamPos) (Variables|Default|GetPlayer2CamPos) (Variables|Default|GetPlayer3CamPos) (Variables|Default|GetPlayer4CamPos)) (Class|VoronoiBlueprints|SnaptoClosest (Utilities|Array|MakeArray (Variables|Default|GetPlayer1Pos) (Variables|Default|GetPlayer2Pos) (Variables|Default|GetPlayer3Pos) (Variables|Default|GetPlayer4Pos)) (Utilities|Array|MakeArray (Variables|Default|GetPlayer1Coord) (Variables|Default|GetPlayer2Coord) (Variables|Default|GetPlayer3Coord) (Variables|Default|GetPlayer4Coord)) (Variables|/Game/Blueprints/SpinTopCharacter.SpinTopCharacter_C|GetPlayerId _array_element_2) (Variables|Default|GetSnapDistance)))) (Class|VoronoiBlueprints|SnapLerpValue (Utilities|Array|Get(acopy) (Utilities|Array|MakeArray (Variables|Default|GetPlayer1Pos) (Variables|Default|GetPlayer2Pos) (Variables|Default|GetPlayer3Pos) (Variables|Default|GetPlayer4Pos)) (Variables|/Game/Blueprints/SpinTopCharacter.SpinTopCharacter_C|GetPlayerId _array_element_2)) (Utilities|Array|Get(acopy) (Utilities|Array|MakeArray (Variables|Default|GetPlayer1Pos) (Variables|Default|GetPlayer2Pos) (Variables|Default|GetPlayer3Pos) (Variables|Default|GetPlayer4Pos)) (Class|VoronoiBlueprints|SnaptoClosest (Utilities|Array|MakeArray (Variables|Default|GetPlayer1Pos) (Variables|Default|GetPlayer2Pos) (Variables|Default|GetPlayer3Pos) (Variables|Default|GetPlayer4Pos)) (Utilities|Array|MakeArray (Variables|Default|GetPlayer1Coord) (Variables|Default|GetPlayer2Coord) (Variables|Default|GetPlayer3Coord) (Variables|Default|GetPlayer4Coord)) (Variables|/Game/Blueprints/SpinTopCharacter.SpinTopCharacter_C|GetPlayerId _array_element_2) (Variables|Default|GetSnapDistance))) (Variables|Default|GetSnapClose) (Variables|Default|GetSnapInterpolation))) false false))
      (:2
        (Transformation|SetWorldLocation (Actor|GetComponentbyClass _array_element_2 "/Script/Engine.SceneCaptureComponent2D") (Math|Vector|Lerp(Vector) (+ (Math|Vector|MakeVector (* (- (.Y (Math|Vector|BreakVector (Utilities|Array|Get(acopy) (Utilities|Array|MakeArray (Variables|Default|GetPlayer1Coord) (Variables|Default|GetPlayer2Coord) (Variables|Default|GetPlayer3Coord) (Variables|Default|GetPlayer4Coord)) (Variables|/Game/Blueprints/SpinTopCharacter.SpinTopCharacter_C|GetPlayerId _array_element_2)))) 0.5) (Variables|Default|GetXCoordinateOffset)) (* (- (- 1.0 (.X (Math|Vector|BreakVector (Utilities|Array|Get(acopy) (Utilities|Array|MakeArray (Variables|Default|GetPlayer1Coord) (Variables|Default|GetPlayer2Coord) (Variables|Default|GetPlayer3Coord) (Variables|Default|GetPlayer4Coord)) (Variables|/Game/Blueprints/SpinTopCharacter.SpinTopCharacter_C|GetPlayerId _array_element_2))))) 0.5) (Variables|Default|GetYCoordinateOffset)) 0.0) (Utilities|Array|Get(acopy) (Utilities|Array|MakeArray (Variables|Default|GetPlayer1CamPos) (Variables|Default|GetPlayer2CamPos) (Variables|Default|GetPlayer3CamPos) (Variables|Default|GetPlayer4CamPos)) (Variables|/Game/Blueprints/SpinTopCharacter.SpinTopCharacter_C|GetPlayerId _array_element_2))) (+ (Math|Vector|MakeVector (* (- (.Y (Math|Vector|BreakVector (Utilities|Array|Get(acopy) (Utilities|Array|MakeArray (Variables|Default|GetPlayer1Coord) (Variables|Default|GetPlayer2Coord) (Variables|Default|GetPlayer3Coord) (Variables|Default|GetPlayer4Coord)) (Class|VoronoiBlueprints|SnaptoClosest (Utilities|Array|MakeArray (Variables|Default|GetPlayer1Pos) (Variables|Default|GetPlayer2Pos) (Variables|Default|GetPlayer3Pos) (Variables|Default|GetPlayer4Pos)) (Utilities|Array|MakeArray (Variables|Default|GetPlayer1Coord) (Variables|Default|GetPlayer2Coord) (Variables|Default|GetPlayer3Coord) (Variables|Default|GetPlayer4Coord)) (Variables|/Game/Blueprints/SpinTopCharacter.SpinTopCharacter_C|GetPlayerId _array_element_2) (Variables|Default|GetSnapDistance))))) 0.5) (Variables|Default|GetXCoordinateOffset)) (* (- (- 1.0 (.X (Math|Vector|BreakVector (Utilities|Array|Get(acopy) (Utilities|Array|MakeArray (Variables|Default|GetPlayer1Coord) (Variables|Default|GetPlayer2Coord) (Variables|Default|GetPlayer3Coord) (Variables|Default|GetPlayer4Coord)) (Class|VoronoiBlueprints|SnaptoClosest (Utilities|Array|MakeArray (Variables|Default|GetPlayer1Pos) (Variables|Default|GetPlayer2Pos) (Variables|Default|GetPlayer3Pos) (Variables|Default|GetPlayer4Pos)) (Utilities|Array|MakeArray (Variables|Default|GetPlayer1Coord) (Variables|Default|GetPlayer2Coord) (Variables|Default|GetPlayer3Coord) (Variables|Default|GetPlayer4Coord)) (Variables|/Game/Blueprints/SpinTopCharacter.SpinTopCharacter_C|GetPlayerId _array_element_2) (Variables|Default|GetSnapDistance)))))) 0.5) (Variables|Default|GetYCoordinateOffset)) 0.0) (Utilities|Array|Get(acopy) (Utilities|Array|MakeArray (Variables|Default|GetPlayer1CamPos) (Variables|Default|GetPlayer2CamPos) (Variables|Default|GetPlayer3CamPos) (Variables|Default|GetPlayer4CamPos)) (Class|VoronoiBlueprints|SnaptoClosest (Utilities|Array|MakeArray (Variables|Default|GetPlayer1Pos) (Variables|Default|GetPlayer2Pos) (Variables|Default|GetPlayer3Pos) (Variables|Default|GetPlayer4Pos)) (Utilities|Array|MakeArray (Variables|Default|GetPlayer1Coord) (Variables|Default|GetPlayer2Coord) (Variables|Default|GetPlayer3Coord) (Variables|Default|GetPlayer4Coord)) (Variables|/Game/Blueprints/SpinTopCharacter.SpinTopCharacter_C|GetPlayerId _array_element_2) (Variables|Default|GetSnapDistance)))) (Class|VoronoiBlueprints|SnapLerpValue (Utilities|Array|Get(acopy) (Utilities|Array|MakeArray (Variables|Default|GetPlayer1Pos) (Variables|Default|GetPlayer2Pos) (Variables|Default|GetPlayer3Pos) (Variables|Default|GetPlayer4Pos)) (Variables|/Game/Blueprints/SpinTopCharacter.SpinTopCharacter_C|GetPlayerId _array_element_2)) (Utilities|Array|Get(acopy) (Utilities|Array|MakeArray (Variables|Default|GetPlayer1Pos) (Variables|Default|GetPlayer2Pos) (Variables|Default|GetPlayer3Pos) (Variables|Default|GetPlayer4Pos)) (Class|VoronoiBlueprints|SnaptoClosest (Utilities|Array|MakeArray (Variables|Default|GetPlayer1Pos) (Variables|Default|GetPlayer2Pos) (Variables|Default|GetPlayer3Pos) (Variables|Default|GetPlayer4Pos)) (Utilities|Array|MakeArray (Variables|Default|GetPlayer1Coord) (Variables|Default|GetPlayer2Coord) (Variables|Default|GetPlayer3Coord) (Variables|Default|GetPlayer4Coord)) (Variables|/Game/Blueprints/SpinTopCharacter.SpinTopCharacter_C|GetPlayerId _array_element_2) (Variables|Default|GetSnapDistance))) (Variables|Default|GetSnapClose) (Variables|Default|GetSnapInterpolation))) false false))
      (:3
        (Transformation|SetWorldLocation (Actor|GetComponentbyClass _array_element_2 "/Script/Engine.SceneCaptureComponent2D") (Math|Vector|Lerp(Vector) (+ (Math|Vector|MakeVector (* (- (.Y (Math|Vector|BreakVector (Utilities|Array|Get(acopy) (Utilities|Array|MakeArray (Variables|Default|GetPlayer1Coord) (Variables|Default|GetPlayer2Coord) (Variables|Default|GetPlayer3Coord) (Variables|Default|GetPlayer4Coord)) (Variables|/Game/Blueprints/SpinTopCharacter.SpinTopCharacter_C|GetPlayerId _array_element_2)))) 0.5) (Variables|Default|GetXCoordinateOffset)) (* (- (- 1.0 (.X (Math|Vector|BreakVector (Utilities|Array|Get(acopy) (Utilities|Array|MakeArray (Variables|Default|GetPlayer1Coord) (Variables|Default|GetPlayer2Coord) (Variables|Default|GetPlayer3Coord) (Variables|Default|GetPlayer4Coord)) (Variables|/Game/Blueprints/SpinTopCharacter.SpinTopCharacter_C|GetPlayerId _array_element_2))))) 0.5) (Variables|Default|GetYCoordinateOffset)) 0.0) (Utilities|Array|Get(acopy) (Utilities|Array|MakeArray (Variables|Default|GetPlayer1CamPos) (Variables|Default|GetPlayer2CamPos) (Variables|Default|GetPlayer3CamPos) (Variables|Default|GetPlayer4CamPos)) (Variables|/Game/Blueprints/SpinTopCharacter.SpinTopCharacter_C|GetPlayerId _array_element_2))) (+ (Math|Vector|MakeVector (* (- (.Y (Math|Vector|BreakVector (Utilities|Array|Get(acopy) (Utilities|Array|MakeArray (Variables|Default|GetPlayer1Coord) (Variables|Default|GetPlayer2Coord) (Variables|Default|GetPlayer3Coord) (Variables|Default|GetPlayer4Coord)) (Class|VoronoiBlueprints|SnaptoClosest (Utilities|Array|MakeArray (Variables|Default|GetPlayer1Pos) (Variables|Default|GetPlayer2Pos) (Variables|Default|GetPlayer3Pos) (Variables|Default|GetPlayer4Pos)) (Utilities|Array|MakeArray (Variables|Default|GetPlayer1Coord) (Variables|Default|GetPlayer2Coord) (Variables|Default|GetPlayer3Coord) (Variables|Default|GetPlayer4Coord)) (Variables|/Game/Blueprints/SpinTopCharacter.SpinTopCharacter_C|GetPlayerId _array_element_2) (Variables|Default|GetSnapDistance))))) 0.5) (Variables|Default|GetXCoordinateOffset)) (* (- (- 1.0 (.X (Math|Vector|BreakVector (Utilities|Array|Get(acopy) (Utilities|Array|MakeArray (Variables|Default|GetPlayer1Coord) (Variables|Default|GetPlayer2Coord) (Variables|Default|GetPlayer3Coord) (Variables|Default|GetPlayer4Coord)) (Class|VoronoiBlueprints|SnaptoClosest (Utilities|Array|MakeArray (Variables|Default|GetPlayer1Pos) (Variables|Default|GetPlayer2Pos) (Variables|Default|GetPlayer3Pos) (Variables|Default|GetPlayer4Pos)) (Utilities|Array|MakeArray (Variables|Default|GetPlayer1Coord) (Variables|Default|GetPlayer2Coord) (Variables|Default|GetPlayer3Coord) (Variables|Default|GetPlayer4Coord)) (Variables|/Game/Blueprints/SpinTopCharacter.SpinTopCharacter_C|GetPlayerId _array_element_2) (Variables|Default|GetSnapDistance)))))) 0.5) (Variables|Default|GetYCoordinateOffset)) 0.0) (Utilities|Array|Get(acopy) (Utilities|Array|MakeArray (Variables|Default|GetPlayer1CamPos) (Variables|Default|GetPlayer2CamPos) (Variables|Default|GetPlayer3CamPos) (Variables|Default|GetPlayer4CamPos)) (Class|VoronoiBlueprints|SnaptoClosest (Utilities|Array|MakeArray (Variables|Default|GetPlayer1Pos) (Variables|Default|GetPlayer2Pos) (Variables|Default|GetPlayer3Pos) (Variables|Default|GetPlayer4Pos)) (Utilities|Array|MakeArray (Variables|Default|GetPlayer1Coord) (Variables|Default|GetPlayer2Coord) (Variables|Default|GetPlayer3Coord) (Variables|Default|GetPlayer4Coord)) (Variables|/Game/Blueprints/SpinTopCharacter.SpinTopCharacter_C|GetPlayerId _array_element_2) (Variables|Default|GetSnapDistance)))) (Class|VoronoiBlueprints|SnapLerpValue (Utilities|Array|Get(acopy) (Utilities|Array|MakeArray (Variables|Default|GetPlayer1Pos) (Variables|Default|GetPlayer2Pos) (Variables|Default|GetPlayer3Pos) (Variables|Default|GetPlayer4Pos)) (Variables|/Game/Blueprints/SpinTopCharacter.SpinTopCharacter_C|GetPlayerId _array_element_2)) (Utilities|Array|Get(acopy) (Utilities|Array|MakeArray (Variables|Default|GetPlayer1Pos) (Variables|Default|GetPlayer2Pos) (Variables|Default|GetPlayer3Pos) (Variables|Default|GetPlayer4Pos)) (Class|VoronoiBlueprints|SnaptoClosest (Utilities|Array|MakeArray (Variables|Default|GetPlayer1Pos) (Variables|Default|GetPlayer2Pos) (Variables|Default|GetPlayer3Pos) (Variables|Default|GetPlayer4Pos)) (Utilities|Array|MakeArray (Variables|Default|GetPlayer1Coord) (Variables|Default|GetPlayer2Coord) (Variables|Default|GetPlayer3Coord) (Variables|Default|GetPlayer4Coord)) (Variables|/Game/Blueprints/SpinTopCharacter.SpinTopCharacter_C|GetPlayerId _array_element_2) (Variables|Default|GetSnapDistance))) (Variables|Default|GetSnapClose) (Variables|Default|GetSnapInterpolation))) false false))))
  (Rendering|Material|SetScalarParameterValue (Variables|Default|GetVoronoi%20Mat) "1-2line" (Class|VoronoiBlueprints|GetLineThickness (Variables|Default|GetPlayer1Pos) (Variables|Default|GetPlayer2Pos) (Variables|Default|GetSnapClose) (Variables|Default|GetThicknessDamping)) :!class /Script/Engine.MaterialInstanceDynamic)
  (Rendering|Material|SetScalarParameterValue (Variables|Default|GetVoronoi%20Mat) "1-3line" (Class|VoronoiBlueprints|GetLineThickness (Variables|Default|GetPlayer1Pos) (Variables|Default|GetPlayer3Pos) (Variables|Default|GetSnapClose) (Variables|Default|GetThicknessDamping)) :!class /Script/Engine.MaterialInstanceDynamic)
  (Rendering|Material|SetScalarParameterValue (Variables|Default|GetVoronoi%20Mat) "1-4line" (Class|VoronoiBlueprints|GetLineThickness (Variables|Default|GetPlayer1Pos) (Variables|Default|GetPlayer4Pos) (Variables|Default|GetSnapClose) (Variables|Default|GetThicknessDamping)) :!class /Script/Engine.MaterialInstanceDynamic)
  (Rendering|Material|SetScalarParameterValue (Variables|Default|GetVoronoi%20Mat) "2-3line" (Class|VoronoiBlueprints|GetLineThickness (Variables|Default|GetPlayer2Pos) (Variables|Default|GetPlayer3Pos) (Variables|Default|GetSnapClose) (Variables|Default|GetThicknessDamping)) :!class /Script/Engine.MaterialInstanceDynamic)
  (Rendering|Material|SetScalarParameterValue (Variables|Default|GetVoronoi%20Mat) "2-4line" (Class|VoronoiBlueprints|GetLineThickness (Variables|Default|GetPlayer2Pos) (Variables|Default|GetPlayer4Pos) (Variables|Default|GetSnapClose) (Variables|Default|GetThicknessDamping)) :!class /Script/Engine.MaterialInstanceDynamic)
  (Rendering|Material|SetScalarParameterValue (Variables|Default|GetVoronoi%20Mat) "3-4line" (Class|VoronoiBlueprints|GetLineThickness (Variables|Default|GetPlayer3Pos) (Variables|Default|GetPlayer4Pos) (Variables|Default|GetSnapClose) (Variables|Default|GetThicknessDamping)) :!class /Script/Engine.MaterialInstanceDynamic))

(fn CalculateVoronoiBounds
  (bind _outactors (Actor|GetAllActorsOfClass "/Game/Blueprints/SpinTopCharacter.SpinTopCharacter_C"))
  (Class|VisualLoggerKismetLibrary|LogText 0 (Utilities|String|ToString(Vector) (Class|VoronoiBlueprints|MinPositionBound _outactors)) "VisLogBP")
  (bind _output_get (Variables|Default|SetMinBound (Class|VoronoiBlueprints|MinPositionBound _outactors)))
  (Class|VisualLoggerKismetLibrary|LogText 0 (Utilities|String|ToString(Vector) (Class|VoronoiBlueprints|MaxPositionBound _outactors)) "VisLogBP")
  (bind _output_get_2 (Variables|Default|SetMaxBound (Class|VoronoiBlueprints|MaxPositionBound _outactors)))
  (Variables|Default|SetXSize (+ 2e+02 (- (.X (Math|Vector|BreakVector _output_get_2)) (.X (Math|Vector|BreakVector _output_get)))))
  (Variables|Default|SetYSize (+ 2e+02 (- (.Y (Math|Vector|BreakVector _output_get_2)) (.Y (Math|Vector|BreakVector _output_get))))))