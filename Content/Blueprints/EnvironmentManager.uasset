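; Environment manager that builds a grid arena of TileBlock01 floor actors and shrinks its bounds over time.
; On BeginPlay it generates the floor, then spawns four scaled WorldSweeper actors just outside the edges.
; A looping timer calls Sweep by name, teleporting each sweeper one grid cell inward per tick.
; PlaceWalls can randomly stack blocks on floor tiles, but its call is disconnected, so it never runs.
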(event EventBeginPlay
  (CallFunction|GenerateWorld)
  (CallFunction|InitializeSweepers)
  (Utilities|Time|SetTimerbyFunctionName 0 "Sweep" (Variables|Default|GetTimeBetweenShrink) true (/ (Variables|Default|GetInitialStartDelay) 8.0)))

(fn ConstructionScript)

(fn GenerateFloor
  (for _index (range 0 (Variables|Default|GetY%20Max))
    (for _index_2 (range 0 (Variables|Default|GetX%20Max))
      (bind _returnvalue (Game|SpawnActorfromClass "/Game/Blueprints/BuildingBlocks/TileBlock01.TileBlock01_C" (Math|Transform|MakeTransform (Math|Vector|MakeVector (Math|Conversions|ToFloat(Integer) (* _index_2 (Variables|Default|GetGridSize))) (Math|Conversions|ToFloat(Integer) (* _index (Variables|Default|GetGridSize))) (Math|Conversions|ToFloat(Integer) (* (Variables|Default|GetGridSize) -1)))) "Undefined" 0 0))
      (Utilities|Array|Add (Variables|Default|GetGroundBlockArray) _returnvalue))))

(fn InitializeSweepers
  (bind _gridsize (Variables|Default|GetGridSize))
  (bind _x_max (Variables|Default|GetX%20Max))
  (bind _gridsize_2 (Variables|Default|GetGridSize))
  (bind _gridsize_3 (Variables|Default|GetGridSize))
  (bind _gridsize_4 (Variables|Default|GetGridSize))
  (bind _x_max_2 (Variables|Default|GetX%20Max))
  (bind _gridsize_5 (Variables|Default|GetGridSize))
  (bind _gridsize_6 (Variables|Default|GetGridSize))
  (bind _gridsize_7 (Variables|Default|GetGridSize))
  (bind _gridsize_8 (Variables|Default|GetGridSize))
  (bind _y_max (Variables|Default|GetY%20Max))
  (bind _gridsize_9 (Variables|Default|GetGridSize))
  (bind _gridsize_10 (Variables|Default|GetGridSize))
  (bind _y_max_2 (Variables|Default|GetY%20Max))
  (bind _returnvalue (+ _x_max 1))
  (bind _returnvalue_2 (* _gridsize_2 2))
  (bind _returnvalue_3 (+ _x_max_2 1))
  (bind _returnvalue_4 (* _gridsize_5 2))
  (bind _returnvalue_5 (+ _y_max 1))
  (bind _returnvalue_6 (* _gridsize_8 2))
  (bind _returnvalue_7 (* _gridsize_9 2))
  (bind _returnvalue_8 (+ _y_max_2 1))
  (bind _returnvalue_9 (Math|Conversions|ToFloat(Integer) _returnvalue_2))
  (bind _returnvalue_10 (Math|Conversions|ToFloat(Integer) _returnvalue_4))
  (bind _returnvalue_11 (Math|Conversions|ToFloat(Integer) _returnvalue_6))
  (bind _returnvalue_12 (Math|Conversions|ToFloat(Integer) _returnvalue_7))
  (bind _returnvalue_13 (* _returnvalue _gridsize))
  (bind _returnvalue_14 (* _returnvalue_3 _gridsize_4))
  (bind _returnvalue_15 (* _returnvalue_5 _gridsize_7))
  (bind _returnvalue_16 (* _returnvalue_8 _gridsize_10))
  (bind _returnvalue_17 (Math|Conversions|ToFloat(Integer) _returnvalue_13))
  (bind _returnvalue_18 (Math|Conversions|ToFloat(Integer) _returnvalue_14))
  (bind _returnvalue_19 (Math|Conversions|ToFloat(Integer) _returnvalue_15))
  (bind _returnvalue_20 (Math|Conversions|ToFloat(Integer) _returnvalue_16))
  (bind _returnvalue_21 (/ _returnvalue_17 2.0))
  (bind _returnvalue_22 (/ _returnvalue_18 2.0))
  (bind _returnvalue_23 (/ _returnvalue_19 2.0))
  (bind _returnvalue_24 (/ _returnvalue_20 2.0))
  (bind _returnvalue_25 (Game|SpawnActorfromClass "/Game/Blueprints/WorldSweeper.WorldSweeper_C" (Math|Transform|MakeTransform (Math|Vector|MakeVector (- _returnvalue_21 (Math|Conversions|ToFloat(Integer) _gridsize_3)) (Math|Conversions|ToFloat(Integer) (* _gridsize_3 -3)) (* (Math|Conversions|ToFloat(Integer) (Variables|Default|GetGridSize)) -0.5)) "0, 0, 0" (Math|Vector|MakeVector _returnvalue_21 _returnvalue_9 _returnvalue_9)) "AlwaysSpawn" 0 0))
  (Variables|Default|SetLeftSweeper _returnvalue_25)
  (bind _returnvalue_26 (Game|SpawnActorfromClass "/Game/Blueprints/WorldSweeper.WorldSweeper_C" (Math|Transform|MakeTransform (Math|Vector|MakeVector (- _returnvalue_22 (Math|Conversions|ToFloat(Integer) _gridsize_6)) (Math|Conversions|ToFloat(Integer) (* _gridsize_6 (+ (Variables|Default|GetY%20Max) 4))) (* (Math|Conversions|ToFloat(Integer) (Variables|Default|GetGridSize)) -0.5)) "0, 0, 0" (Math|Vector|MakeVector _returnvalue_22 _returnvalue_10 _returnvalue_10)) "AlwaysSpawn" 0 0))
  (Variables|Default|SetRightSweeper _returnvalue_26)
  (bind _returnvalue_27 (Game|SpawnActorfromClass "/Game/Blueprints/WorldSweeper.WorldSweeper_C" (Math|Transform|MakeTransform (Math|Vector|MakeVector (Math|Conversions|ToFloat(Integer) (* (Variables|Default|GetGridSize) (+ (Variables|Default|GetX%20Max) 3))) _returnvalue_24 (* (Math|Conversions|ToFloat(Integer) (Variables|Default|GetGridSize)) -0.5)) "0, 0, 0" (Math|Vector|MakeVector _returnvalue_12 _returnvalue_24 _returnvalue_12)) "AlwaysSpawn" 0 0))
  (Variables|Default|SetTopSweeper _returnvalue_27)
  (bind _returnvalue_28 (Game|SpawnActorfromClass "/Game/Blueprints/WorldSweeper.WorldSweeper_C" (Math|Transform|MakeTransform (Math|Vector|MakeVector (Math|Conversions|ToFloat(Integer) (* (Variables|Default|GetGridSize) -4)) _returnvalue_23 (* (Math|Conversions|ToFloat(Integer) (Variables|Default|GetGridSize)) -0.5)) "0, 0, 0" (Math|Vector|MakeVector _returnvalue_11 _returnvalue_23 _returnvalue_11)) "AlwaysSpawn" 0 0))
  (Variables|Default|SetBottomSweeper _returnvalue_28))

(fn Sweep
  (bind _bottomsweeper (Variables|Default|GetBottomSweeper))
  (bind _leftsweeper (Variables|Default|GetLeftSweeper))
  (bind _rightsweeper (Variables|Default|GetRightSweeper))
  (bind _topsweeper (Variables|Default|GetTopSweeper))
  (bind _returnvalue (Transformation|GetActorLocation _bottomsweeper))
  (bind _returnvalue_2 (Transformation|GetActorLocation _rightsweeper))
  (bind _returnvalue_3 (Transformation|GetActorLocation _topsweeper))
  (bind _returnvalue_4 (Transformation|GetActorLocation _leftsweeper))
  (bind (_x _y _z) (Math|Vector|BreakVector _returnvalue_2))
  (bind (_x_2 _y_2 _z_2) (Math|Vector|BreakVector _returnvalue_3))
  (bind (_x_3 _y_3 _z_3) (Math|Vector|BreakVector _returnvalue))
  (bind (_x_4 _y_4 _z_4) (Math|Vector|BreakVector _returnvalue_4))
  (Transformation|Teleport _leftsweeper (Math|Vector|MakeVector _x_4 (+ _y_4 (Math|Conversions|ToFloat(Integer) (Variables|Default|GetGridSize))) _z_4) "0, 0, 0")
  (Transformation|Teleport _rightsweeper (Math|Vector|MakeVector _x (- _y (Math|Conversions|ToFloat(Integer) (Variables|Default|GetGridSize))) _z) "0, 0, 0")
  (Transformation|Teleport _topsweeper (Math|Vector|MakeVector (- _x_2 (Math|Conversions|ToFloat(Integer) (Variables|Default|GetGridSize))) _y_2 _z_2) "0, 0, 0")
  (Transformation|Teleport _bottomsweeper (Math|Vector|MakeVector (+ _x_3 (Math|Conversions|ToFloat(Integer) (Variables|Default|GetGridSize))) _y_3 _z_3) "0, 0, 0"))

(fn GenerateWorld
  (CallFunction|GenerateFloor))

(fn PlaceWalls
  (for (_array_element _array_index) (Variables|Default|GetGroundBlockArray)
    (LocalVariables|SetCurrentFloorActor _array_element)
    (LocalVariables|SetCurrentIndex _array_index)
    (if (<= (Math|Random|RandomFloatinRange 0.0 1.0) (Variables|Default|GetWallProbability))
      (if (not (.ReturnValue (Utilities|Map|Find (Variables|Default|GetOccupiedSpaces) (LocalVariables|GetCurrentIndex))))
        (bind _returnvalue (Game|SpawnActorfromClass "/Game/Blueprints/BuildingBlocks/TileBlock01.TileBlock01_C" (Math|Transform|MakeTransform (Math|Vector|MakeVector (.X (Math|Vector|BreakVector (Transformation|GetActorLocation (LocalVariables|GetCurrentFloorActor)))) (.Y (Math|Vector|BreakVector (Transformation|GetActorLocation (LocalVariables|GetCurrentFloorActor)))) (+ (.Z (Math|Vector|BreakVector (Transformation|GetActorLocation (LocalVariables|GetCurrentFloorActor)))) (Math|Conversions|ToFloat(Integer) (Variables|Default|GetGridSize))))) "Undefined" 0 0))
        (Variables|Default|SetOccupiedSpaces (Utilities|Map|MakeMap (LocalVariables|GetCurrentIndex) _returnvalue))))))