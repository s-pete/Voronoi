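; TilingBlock is a building-block Blueprint whose cube mesh shows a configurable debug edge highlight.
; The construction script writes the highlight color, scaled by its alpha, and the edge ratio to the cube's material parameters.
; On BeginPlay, the highlight color is set to black unless RenderHighlightInGame is enabled.
; DropTheBlock is an empty function.
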(event EventBeginPlay
  (if (not (Variables|Default|GetRender%20highlight%20in%20game))
    (Rendering|Material|SetVectorParameterValueonMaterials (Variables|Default|GetSM_Cube) "Debug Edge Highlight" "0, 0, 0")))

(fn ConstructionScript
  (bind _highlight_color (Variables|Default|GetHighlight%20color))
  (bind (_r _g _b _a) (Math|Color|BreakColor _highlight_color))
  (Rendering|Material|SetVectorParameterValueonMaterials (Variables|Default|GetSM_Cube) "Debug Edge Highlight" (* (Math|Vector|MakeVector _r _g _b) _a))
  (Rendering|Material|SetScalarParameterValueonMaterials (Variables|Default|GetSM_Cube) "Debug Edge Percentage" (Variables|Default|GetHighlight%20ratio)))

(fn DroptheBlock)