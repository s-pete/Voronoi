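; HalfCubeLights01 is a half-cube building block that warns with a red flash and then falls after a WorldSweeper overlaps it.
; The overlap starts a TimeToFall timer, during which Tick drives the dynamic material's RedFlash parameter with a sine of the elapsed time.
; When the timer fires, DropBlock enables physics on the mesh and applies a small downward force.
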(event EventBeginPlay
  (bind _returnvalue (Rendering|Material|CreateDynamicMaterialInstance (Variables|Default|GetSM_Cube_Half_Lights) 0 0 "None" :!class /Script/Engine.PrimitiveComponent))
  (Variables|Default|SetFlashingMaterial _returnvalue))

(event Collision|EventActorBeginOverlap
  (params (OtherActor :type Actor%20Object%20Reference))
  (bind _returnvalue (Utilities|GetClass OtherActor))
  (Development|PrintString (Utilities|GetClassDisplayName _returnvalue))
  (if (== _returnvalue "/Game/Blueprints/WorldSweeper.WorldSweeper_C")
    (bind _returnvalue_2 (Utilities|Time|SetTimerbyFunctionName 0 "DropBlock" (Variables|Default|GetTimeToFall)))
    (Variables|Default|SetTimeUntilFall _returnvalue_2)
    (Variables|Default|SetCountdownActive true)))

(event EventTick
  (params (DeltaSeconds :type Float%20%28single-precision%29))
  (if (Variables|Default|GetCountdownActive)
    (Rendering|Material|SetVectorParameterValue (Variables|Default|GetFlashingMaterial) "RedFlash" (Utilities|Struct|MakeLinearColor (/ (Math|Float|Absolute(Float) (Math|Trig|Sin(Radians) (* (Class|KismetSystemLibrary|GetTimerElapsedTimeHandle (Variables|Default|GetTimeUntilFall)) (Variables|Default|GetTimeToFall) 0.5))) 6.66) 0.0 0.0 0.0) :!class /Script/Engine.MaterialInstanceDynamic)))

(fn ConstructionScript)

(fn DropBlock
  (bind _sm_cube_half_lights (Variables|Default|GetSM_Cube_Half_Lights))
  (Development|PrintString "Print")
  (Physics|SetSimulatePhysics _sm_cube_half_lights true)
  (Physics|AddForce _sm_cube_half_lights "0, 0,-10.000000" "None" false))