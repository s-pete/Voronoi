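; Tiling building-block Blueprint for the top half of a ramp, with a debug edge highlight on its mesh materials.
; The construction script passes the highlight color, scaled by its alpha, and an edge percentage to the material parameters.
; BeginPlay sets the highlight to black, so the debug tint is cleared during play.
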(event EventBeginPlay
  (Rendering|Material|SetVectorParameterValueonMaterials (Variables|Default|GetSM_Ramp_Half_Top) "Debug Edge Highlight" "0, 0, 0"))

(fn ConstructionScript
  (bind _debug_edge_highlight (Variables|Default|GetDebug%20Edge%20Highlight))
  (bind (_r _g _b _a) (Math|Color|BreakColor _debug_edge_highlight))
  (Rendering|Material|SetVectorParameterValueonMaterials (Variables|Default|GetSM_Ramp_Half_Top) "Debug Edge Highlight" (* (Math|Vector|MakeVector _r _g _b) _a))
  (Rendering|Material|SetScalarParameterValueonMaterials (Variables|Default|GetSM_Ramp_Half_Top) "Debug Edge Percentage" (Variables|Default|GetDebug%20Edge%20Percentage)))