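; A half-ramp top building block that falls away after a WorldSweeper actor overlaps it.
; The overlap starts a TimeToFall timer, during which Tick drives a sine-based red flash on a dynamic material instance from the timer's elapsed time.
; When the timer expires, DropBlock enables physics on the mesh and pushes it downward with a force and a set velocity.
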(event EventBeginPlay
  (bind _returnvalue (Rendering|Material|CreateDynamicMaterialInstance (Variables|Default|GetSM_Ramp_Half_Top) 1 0 "None" :!class /Script/Engine.PrimitiveComponent))
  (Variables|Default|SetFlashingMaterial _returnvalue))

(event Collision|EventActorBeginOverlap
  (params (OtherActor :type Actor%20Object%20Reference))
  (if (== (Utilities|GetClass OtherActor) "/Game/Blueprints/WorldSweeper.WorldSweeper_C")
    (bind _returnvalue (Utilities|Time|SetTimerbyFunctionName 0 "DropBlock" (Variables|Default|GetTimeToFall)))
    (Variables|Default|SetTimeUntilFall _returnvalue)
    (Variables|Default|SetCountdownActive true)))

(event EventTick
  (params (DeltaSeconds :type Float%20%28single-precision%29))
  (if (Variables|Default|GetCountdownActive)
    (Rendering|Material|SetVectorParameterValue (Variables|Default|GetFlashingMaterial) "RedFlash" (Utilities|Struct|MakeLinearColor (/ (Math|Float|Absolute(Float) (Math|Trig|Sin(Radians) (* (Class|KismetSystemLibrary|GetTimerElapsedTimeHandle (Variables|Default|GetTimeUntilFall)) (Variables|Default|GetTimeToFall) 0.5))) 6.66) 0.0 0.0 0.0) :!class /Script/Engine.MaterialInstanceDynamic)))

(fn ConstructionScript)

(fn DropBlock
  (bind _sm_ramp_half_top (Variables|Default|GetSM_Ramp_Half_Top))
  (Physics|SetSimulatePhysics _sm_ramp_half_top true)
  (Physics|AddForce _sm_ramp_half_top "0, 0,-10.000000" "None" false)
  (Physics|SetPhysicsLinearVelocity _sm_ramp_half_top "0, 0,-1000.000000" false "None"))