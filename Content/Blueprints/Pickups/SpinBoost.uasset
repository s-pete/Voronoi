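; SpinBoost is a respawning pickup that adds a fixed amount of spin to an overlapping SpinTopCharacter, capped at its MaxSpin.
; On pickup it hides and disables its collision, then a timer restores both after RespawnTime.
; Tick yaws the Scene component at ArrowSpinSpeed for a spinning visual.
; The construction script gives the decal a dynamic material instance driven by the size and color variables.
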(event Custom|ToggleActive
  (Rendering|SetActorHiddenInGame false)
  (Collision|SetActorEnableCollision true))

(event Collision|EventActorBeginOverlap
  (params (OtherActor :type Actor%20Object%20Reference))
  (bind _asspin_top_character (Utilities|Casting|CastToSpinTopCharacter OtherActor))
  (Variables|/Game/Blueprints/SpinTopCharacter.SpinTopCharacter_C|SetSpin _asspin_top_character (Math|Float|Clamp(Float) (+ (Variables|/Game/Blueprints/SpinTopCharacter.SpinTopCharacter_C|GetSpin _asspin_top_character) 6e+02) 0.0 (Variables|/Game/Blueprints/SpinTopCharacter.SpinTopCharacter_C|GetMaxSpin _asspin_top_character)))
  (Rendering|SetActorHiddenInGame true)
  (Collision|SetActorEnableCollision false)
  (Utilities|Time|SetTimerbyEvent (delegate Custom|ToggleActive) (Variables|Default|GetRespawnTime)))

(event EventTick
  (params (DeltaSeconds :type Float%20%28single-precision%29))
  (bind _result (Math|Float|NegateFloat DeltaSeconds)
    (:%20%20
      (Transformation|AddLocalRotation (Variables|Default|GetScene) (Math|Rotator|MakeRotator 0.0 0.0 (* _result (Variables|Default|GetArrow%20spin%20speed))) false false))))

(fn ConstructionScript
  (bind _returnvalue (Rendering|Material|CreateDynamicMaterialInstance (Class|DecalComponent|GetDecalMaterial (Variables|Default|GetDecal)) "None" :!class /Script/Engine.KismetMaterialLibrary))
  (Rendering|Material|SetScalarParameterValue _returnvalue "Additive Size" (Variables|Default|GetAdditive%20decal%20size) :!class /Script/Engine.MaterialInstanceDynamic)
  (Rendering|Material|SetScalarParameterValue _returnvalue "Multiplicative Size" (Variables|Default|GetMultiplicative%20decal%20size) :!class /Script/Engine.MaterialInstanceDynamic)
  (Rendering|Material|SetVectorParameterValue _returnvalue "Color" (Variables|Default|GetDecal%20color) :!class /Script/Engine.MaterialInstanceDynamic)
  (Rendering|Components|Decal|SetDecalMaterial (Variables|Default|GetDecal) _returnvalue))