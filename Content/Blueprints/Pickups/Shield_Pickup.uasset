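; Shield pickup that gives an overlapping SpinTopCharacter a Bounce_Shield, spawned and attached to that character.
; After pickup it hides and disables collision, then a timer restores it after RespawnTime.
; Tick spins two orbiting visual components at separate configurable rates.
; The construction script sets their emissive color and intensity and builds a dynamic decal material with configurable size, color and oscillation, using a random phase offset per instance.
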(event Custom|ToggleActive
  ;[1 1 1] Respawn timer
  (Rendering|SetActorHiddenInGame false)
  (Collision|SetActorEnableCollision true))

(event Collision|EventActorBeginOverlap
  (params (OtherActor :type Actor%20Object%20Reference))
  (bind _asspin_top_character (Utilities|Casting|CastToSpinTopCharacter OtherActor))
  (bind _returnvalue (Game|SpawnActorfromClass "/Game/Blueprints/Pickups/Bounce_Shield.Bounce_Shield_C" (Math|Transform|MakeTransform "0, 0, 0") "AlwaysSpawn" 0 0))
  (Transformation|AttachActorToActor _returnvalue _asspin_top_character "None" "KeepRelative" "KeepRelative" "KeepRelative" true)
  ;[1 1 1] Respawn timer
  (Rendering|SetActorHiddenInGame true)
  (Collision|SetActorEnableCollision false)
  (Utilities|Time|SetTimerbyEvent (delegate Custom|ToggleActive) (Variables|Default|GetRespawnTime)))

(event EventTick
  (params (DeltaSeconds :type Float%20%28single-precision%29))
  (Transformation|AddWorldRotation (Variables|Default|GetOrbiting1) (* (Variables|Default|GetVisual%20rotation%20per%20second%201) DeltaSeconds) false false)
  (Transformation|AddWorldRotation (Variables|Default|GetOrbiting2) (* (Variables|Default|GetVisual%20rotation%20per%20second%202) DeltaSeconds) false false))

(fn ConstructionScript
  (bind _emissive_color (Variables|Default|GetEmissive%20color))
  (bind _returnvalue (Rendering|Material|CreateDynamicMaterialInstance (Class|DecalComponent|GetDecalMaterial (Variables|Default|GetDecal)) "None" :!class /Script/Engine.KismetMaterialLibrary))
  (Rendering|Material|SetScalarParameterValue _returnvalue "Additive Size" (Variables|Default|GetAdditive%20decal%20size) :!class /Script/Engine.MaterialInstanceDynamic)
  (Rendering|Material|SetScalarParameterValue _returnvalue "Multiplicative Size" (Variables|Default|GetMultiplicative%20decal%20size) :!class /Script/Engine.MaterialInstanceDynamic)
  (Rendering|Material|SetScalarParameterValue _returnvalue "Oscilation Speed" (Variables|Default|GetOscilation%20speed) :!class /Script/Engine.MaterialInstanceDynamic)
  (Rendering|Material|SetScalarParameterValue _returnvalue "Oscilation Offset" (Math|Random|RandomFloatinRange 0.0 (Math|Trig|GetPI)) :!class /Script/Engine.MaterialInstanceDynamic)
  (Rendering|Material|SetVectorParameterValue _returnvalue "Color" (Variables|Default|GetDecal%20color) :!class /Script/Engine.MaterialInstanceDynamic)
  (Rendering|Components|Decal|SetDecalMaterial (Variables|Default|GetDecal) _returnvalue)
  (Rendering|Material|SetVectorParameterValueonMaterials (Variables|Default|GetOrbiting1) "MAT_EMISSIVE_COLOR" (* (Math|Vector|MakeVector (.r _emissive_color) (.g _emissive_color) (.b _emissive_color)) (.a _emissive_color)))
  (Rendering|Material|SetScalarParameterValueonMaterials (Variables|Default|GetOrbiting1) "MAT_EMISSIVE_INTENSITY" (Variables|Default|GetEmissive%20intensity)))