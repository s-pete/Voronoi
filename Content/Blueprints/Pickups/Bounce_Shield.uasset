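; Bounce shield actor that pushes overlapping SpinTopCharacters away from its center and destroys itself after ten seconds.
; Each Tick it spins its particle system and applies a horizontal, mass-independent force to those characters' capsules, directed away from the static mesh and skipping any at dead center.
; The construction script tints the mesh materials' emissive parameter from EmissiveColor, using alpha as intensity.
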(event Custom|DestroyOnTimer
  (Actor|DestroyActor))

(event EventBeginPlay
  (Utilities|Time|SetTimerbyEvent (delegate Custom|DestroyOnTimer) 1e+01))

(event Collision|EventActorBeginOverlap
  (params (OtherActor :type Actor%20Object%20Reference)))

(event EventTick
  (params (DeltaSeconds :type Float%20%28single-precision%29))
  (Transformation|AddLocalRotation (Variables|Default|GetParticleSystem) (Math|Rotator|MakeRotator 0.0 0.0 (* DeltaSeconds (Variables|Default|GetParticle%20rotation%20per%20second))) false false)
  (for _array_element (Collision|GetOverlappingActors "/Game/Blueprints/SpinTopCharacter.SpinTopCharacter_C" :!class /Script/Engine.Actor)
    (Math|Float|CompareFloat (Math|Vector|VectorLengthXY (- (Transformation|GetActorLocation _array_element) (Transformation|GetWorldLocation (Variables|Default|GetStaticMesh)))) 0.01
      (:>
        (Physics|AddForce (Actor|GetComponentsByClass _array_element "/Script/Engine.CapsuleComponent") (* (Class|KismetMathLibrary|VectorNormal2D (- (Transformation|GetActorLocation _array_element) (Transformation|GetWorldLocation (Variables|Default|GetStaticMesh))) 0.0001) 5e+03) "None" true)))))

(fn ConstructionScript
  (bind _emissive_color (Variables|Default|GetEmissive%20color))
  (Rendering|Material|SetVectorParameterValueonMaterials (Variables|Default|GetStaticMesh) "MAT_EMISSIVE_COLOR" (* (Math|Vector|MakeVector (.r _emissive_color) (.g _emissive_color) (.b _emissive_color)) (.a _emissive_color))))