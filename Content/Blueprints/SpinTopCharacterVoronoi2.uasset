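; Spinning-top player character for up to four players, each assigned an ID and scene-capture render target by actor count at construction.
; Tick feeds stick input into physics movement that steers velocity while keeping speed, adds force unless stunned, and updates the spin widget.
; Wall hits convert stored Spin into knockback and brief stun, while ramp impulses are clamped against launching.
; Code feeding player positions to the Voronoi split-screen material is disconnected.
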(event EventTick
  (params (DeltaSeconds :type Float%20%28single-precision%29))
  ;[1 1 1] Grab Controller Values and Save For This Frame
  (bind _outputmovement (CallFunction|GetMovementValues))
  (Variables|Default|SetCurrentFrameMovementValues _outputmovement)
  (CallFunction|UpdatePlayerSpinUI)
  (Variables|Default|SetStun (- (Variables|Default|GetStun) DeltaSeconds))
  (CallFunction|MovePlayer))

(event EventBeginPlay
  (bind _camera1 (Variables|Default|GetCamera1))
  ;[1 1 1] Ensure Camera Is Axis Aligned
  (Components|Activation|Activate _camera1 false)
  (Transformation|SetWorldRotation _camera1 "-90.000000, 0, 0" false false))

(event Collision|EventHit
  (params (MyComp :type Primitive%20Component%20Object%20Reference) (Other :type Actor%20Object%20Reference) (OtherComp :type Primitive%20Component%20Object%20Reference) (bSelfMoved :type Boolean) (HitLocation :type Vector :default "0, 0, 0") (HitNormal :type Vector :default "0, 0, 0") (NormalImpulse :type Vector :default "0, 0, 0") (Hit :type Hit%20Result%20Structure%20%28by%20ref%29))
  (CallFunction|HandleNonFloorCollision OtherComp HitNormal NormalImpulse))

(fn ConstructionScript
  (bind _returnvalue (Actor|GetComponentbyClass "/Script/Engine.SceneCaptureComponent2D"))
  (bind _outactors (Actor|GetAllActorsOfClass "/Game/Blueprints/SpinTopCharacterVoronoi.SpinTopCharacterVoronoi_C"))
  (bind _output_get (Variables|Default|SetPlayerId (- (Utilities|Array|Length _outactors) 1)))
  (switch int _output_get
    (:0
      (Variables|/Script/Engine.SceneCaptureComponent2D|SetTextureTarget _returnvalue "/Game/Materials/Player1.Player1"))
    (:1
      (Variables|/Script/Engine.SceneCaptureComponent2D|SetTextureTarget _returnvalue "/Game/Materials/Player2.Player2"))
    (:2
      (Variables|/Script/Engine.SceneCaptureComponent2D|SetTextureTarget _returnvalue "/Game/Materials/Player3.Player3"))
    (:3
      (Variables|/Script/Engine.SceneCaptureComponent2D|SetTextureTarget _returnvalue "/Game/Materials/Player4.Player4"))))

(fn UpdatePlayerSpinUI
  ;[1 1 1] This Shouldn't Fail
  (bind _asplayer_world_ui (Utilities|Casting|CastToPlayerWorldUI (UserInterface|GetUserWidgetObject (Variables|Default|GetSpinWidget))))
  (Variables|/Game/Blueprints/PlayerWorldUI.PlayerWorldUI_C|SetMaxSpinCharge _asplayer_world_ui (Variables|Default|GetMaxSpin))
  (Variables|/Game/Blueprints/PlayerWorldUI.PlayerWorldUI_C|SetCurrentSpinCharge _asplayer_world_ui (Variables|Default|GetSpin)))

(fn GetMovementValues
  (return (Math|Vector|ClampVectorSize (+ (Math|Vector|MakeVector (Input|AxisValues|GetLeftStickY) 0.0 0.0) (Math|Vector|MakeVector 0.0 (Input|AxisValues|GetLeftStickX) 0.0)) 0.0 1.0)))

(fn MovePlayer
  (bind _returnvalue (Transformation|GetVelocity))
  (bind _returnvalue_2 (* _returnvalue "1.000000,1.000000, 0"))
  (bind _returnvalue_3 (Math|Vector|VectorLength _returnvalue_2))
  (if (> (Math|Vector|VectorLength (Variables|Default|GetCurrentFrameMovementValues)) 0.1)
    (if (> _returnvalue_3 0.1)
      (Math|Float|CompareFloat (Class|KismetMathLibrary|DegAcos (Class|KismetMathLibrary|VectorCosineAngle2D _returnvalue_2 (Variables|Default|GetCurrentFrameMovementValues))) 1.2e+02
        (:>
          (Math|Float|CompareFloat (Variables|Default|GetStun) 0.0 :!label _label
            (:==
              _)
            (:<
              _)))
        (:==
          (goto _label))
        (:<
          (Physics|SetPhysicsLinearVelocity (Variables|Collision|GetCapsuleComponent) (+ (* _returnvalue "0.000000,0.000000,1.000000") (* (Math|Vector|Normalize (Math|Vector|Lerp(Vector) (Math|Vector|Normalize _returnvalue_2) (Variables|Default|GetCurrentFrameMovementValues) 0.1)) _returnvalue_3)) false "None")))
      (else
        (goto _label)))
    (else
      (goto _label)))
  (Physics|AddForce (Variables|Collision|GetCapsuleComponent) (* (Variables|Default|GetCurrentFrameMovementValues) 1.5e+03) "None" true))

(fn HandleNonFloorCollision
  (params (FloorComp :type Primitive%20Component%20Object%20Reference) (HitNormal :type Vector) (ImpulseNormal :type Vector))
  (bind _returnvalue (* HitNormal "1.000000,1.000000, 0"))
  (bind _capsulecomponent (Variables|Collision|GetCapsuleComponent))
  (if (Math|Vector|VectorIsNearlyZero _returnvalue 0.7) ; Ignore mostly vertical normals
    (if (not (Math|Vector|VectorIsNearlyZero _returnvalue 0.05)) ; stop "ramp bounce"
      (Physics|AddImpulse _capsulecomponent (- (Math|Vector|ClampVectorSize ImpulseNormal 0.0 0.25) ImpulseNormal) "None" false) ; Add spin impulse
    )
    (else
      (Physics|AddImpulse _capsulecomponent (* (Math|Vector|Normalize _returnvalue) (Math|Float|Clamp(Float) (Variables|Default|GetSpin) 0.0 1e+03)) "None" true) ; Add spin impulse
      (Variables|Default|SetSpin (- (Variables|Default|GetSpin) (Math|Float|Clamp(Float) (Variables|Default|GetSpin) 0.0 1e+03)))
      (Variables|Default|SetStun 0.2) ; "stun" prevents us from moving towards collisions
    )))